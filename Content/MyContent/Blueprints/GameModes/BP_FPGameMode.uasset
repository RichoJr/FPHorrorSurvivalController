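; First-person game mode that records a camera player spawn point and drives a video camera countdown on the HUD.
; On BeginPlay it finds spawn target points, caches the player controller and writes the first point's transform into the camera save slot.
; StartCamTimer lets Tick decrement CamTimer and update the crosshair widget's progress bar, while the timer text shows frame delta seconds.
; The timer expiry and reset logic is unconnected.
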(event Custom|StartCamTimer
  (Variables|Default|SetCamRunning true))

(event EventBeginPlay
  (Utilities|FlowControl|Sequence
    (:then_0
      (bind _astarget_point (Utilities|Casting|CastToTargetPointClass "/Game/MyContent/Blueprints/Player/bp_CamPlayerSpawn.bp_CamPlayerSpawn_C"))
      (bind _outactors (Actor|GetAllActorsOfClass _astarget_point))
      (Variables|Default|SetSpawnPoints _outactors))
    (:then_1
      (bind _output_get (Variables|Default|SetCamPlayerSpawnPoint (Utilities|Array|Get(acopy) (Variables|Default|GetSpawnPoints))))
      (Variables|Default|SetCamPlayerTransform (Transformation|GetActorTransform _output_get)))
    (:then_2
      (bind _asbp_player_controller (Utilities|Casting|CastTobp_PlayerController (Game|GetPlayerController 0)))
      (Variables|Default|SetMyPlayerController _asbp_player_controller))
    (:then_3
      (bind _returnvalue (SaveGame|LoadGamefromSlot (Variables|Default|GetCamSaveName)))
      (bind _asbp_camera_saves (Utilities|Casting|CastTobp_CameraSaves _returnvalue))
      (bind _output_get_2 (Variables|Default|SetCamSave _asbp_camera_saves))
      (Variables|/Game/MyContent/Blueprints/Saves/bp_CameraSaves.bp_CameraSaves_C|SetcamPlayer1 _output_get_2 (Variables|Default|GetCamPlayerTransform))
      (SaveGame|SaveGametoSlot _output_get_2 (Variables|Default|GetCamSaveName)))))

(event EventTick
  (params (DeltaSeconds :type Float%20%28single-precision%29))
  (bind _returnvalue (Utilities|Time|GetWorldDeltaSeconds))
  (bind _myplayercontroller (Variables|Default|GetMyPlayerController))
  (bind _worldplayer (Variables|/Game/MyContent/Blueprints/Player/bp_PlayerController.bp_PlayerController_C|GetworldPlayer _myplayercontroller))
  (bind _crosshairref (Variables|/Game/MyContent/Blueprints/Player/bp_PlayerCharacter.bp_PlayerCharacter_C|GetCrosshairRef _worldplayer))
  (if (Variables|Default|GetCamRunning)
    (Variables|/Script/UMG.TextBlock|SetText (Variables|/Game/MyContent/Blueprints/UI/Widgets/WBP_Crosshair.WBP_Crosshair_C|GetVideo_TimerText _crosshairref) (Utilities|Text|ToText(Float) _returnvalue "HalfToEven"))
    (bind _output_get (Variables|Default|SetCamTimer (- (Variables|Default|GetCamTimer) _returnvalue)))
    (Progress|SetPercent (Variables|/Game/MyContent/Blueprints/UI/Widgets/WBP_Crosshair.WBP_Crosshair_C|GetVideo_ProgressBar _crosshairref) _output_get)))

(fn ConstructionScript)