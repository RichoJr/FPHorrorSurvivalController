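; Interactable camcorder actor that switches the player into a camera screen through the player controller.
; On BeginPlay it caches the player controller and writes its transform to the CamCord1Save field of an existing camera save game.
; CameraInteract calls SwitchPlayerCharacter with its Screen, stores the result as the on state, then after a short timer passes that state to the controller's camera screen UI.
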(event Custom|Turn%20on%20UI
  (Default|CameraScreenUIActive (Variables|Default|GetplayerController) (stale EventCameraInteract _output_get)))

(event EventCameraInteract
  (Development|PrintString (Utilities|GetDisplayName self))
  (bind _camon (Default|SwitchPlayerCharacter (Variables|Default|GetplayerController) (Variables|Default|GetScreen)))
  (bind _output_get (Variables|Default|SetCam%20On _camon))
  (Utilities|Time|SetTimerbyEvent (delegate Custom|Turn%20on%20UI) 0.75))

(event EventBeginPlay
  (Utilities|FlowControl|Sequence
    (:then_0
      (bind _asbp_player_controller (Utilities|Casting|CastTobp_PlayerController (Game|GetPlayerController 0)))
      (Variables|Default|SetplayerController _asbp_player_controller))
    (:then_1
      (Variables|Default|SetcamSaveTransform (Transformation|GetActorTransform)))
    (:then_2
      (bind _returnvalue (SaveGame|LoadGamefromSlot (Variables|Default|Getbp_CameraSaves)))
      (bind _asbp_camera_saves (Utilities|Casting|CastTobp_CameraSaves _returnvalue))
      (bind _output_get (Variables|Default|SetCameraLocationSave _asbp_camera_saves))
      (Variables|/Game/MyContent/Blueprints/Saves/bp_CameraSaves.bp_CameraSaves_C|SetCamCord1Save _output_get (Variables|Default|GetcamSaveTransform))
      (SaveGame|SaveGametoSlot (Variables|Default|GetCameraLocationSave) (Variables|Default|Getbp_CameraSaves)))))

(fn ConstructionScript)