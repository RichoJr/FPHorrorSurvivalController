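; Player-side Blueprint for camera mode that handles closing the camera and restoring saved transforms.
; The close input loads the camcorder and transforms from a save slot, then has the player controller switch character and update the camera screen UI.
; Tick eases the camcorder toward its saved transform with TInterpTo until a one-second timer ends the blend and snaps this actor to the saved player transform.
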(event Custom|Closed
  (Variables|Default|SetCloseCamera false)
  (Transformation|SetActorTransform (stale Input|EnhancedActionEvents|EnhancedInputActionIA_CloseCamera _playertransform)))

(event Input|EnhancedActionEvents|EnhancedInputActionIA_CloseCamera
  (params (ActionValue :type Boolean) (ElapsedSeconds :type Float%20%28double-precision%29) (TriggeredSeconds :type Float%20%28double-precision%29) (InputAction :type Input%20Action%20Object%20Reference :default "/Game/MyContent/Inputs/Actions/IA_CloseCamera.IA_CloseCamera"))
  (bind _playercontroller (Variables|Default|GetPlayerController))
  (:Started
    (Development|PrintString "Close")
    (Variables|Default|SetCloseCamera true)
    (bind (_camcorder _camtransform _playertransform) (CallFunction|LoadCamTransformSave))
    (bind _camon (Default|SwitchPlayerCharacter _playercontroller))
    (Default|CameraScreenUIActive _playercontroller _camon)
    (Utilities|Time|SetTimerbyEvent (delegate Custom|Closed) 1.0)))

(event EventBeginPlay
  (|CallParentFunction)
  (bind _asbp_player_controller (Utilities|Casting|CastTobp_PlayerController (Game|GetPlayerController 0)))
  (Variables|Default|SetPlayerController _asbp_player_controller))

(event Collision|EventActorBeginOverlap
  (params (OtherActor :type Actor%20Object%20Reference)))

(event EventTick
  (params (DeltaSeconds :type Float%20%28single-precision%29))
  (|CallParentFunction DeltaSeconds)
  (if (Variables|Default|GetCloseCamera)
    (Transformation|SetActorTransform (stale Input|EnhancedActionEvents|EnhancedInputActionIA_CloseCamera _camcorder) (Class|KismetMathLibrary|TInterpto (Transformation|GetActorTransform (stale Input|EnhancedActionEvents|EnhancedInputActionIA_CloseCamera _camcorder)) (stale Input|EnhancedActionEvents|EnhancedInputActionIA_CloseCamera _camtransform) (Utilities|Time|GetWorldDeltaSeconds) 5.0))))

(fn ConstructionScript
  (|CallParentFunction))

(fn LoadCamTransformSave
  (bind _returnvalue (SaveGame|LoadGamefromSlot (LocalVariables|GetCamSaveName)))
  (bind _asbp_camera_saves (Utilities|Casting|CastTobp_CameraSaves _returnvalue))
  (bind _output_get (LocalVariables|SetCamCaves _asbp_camera_saves))
  (bind _output_get_2 (LocalVariables|SetCamCordObject (Variables|/Game/MyContent/Blueprints/Saves/bp_CameraSaves.bp_CameraSaves_C|GetCamCord1 _output_get)))
  (bind _output_get_3 (LocalVariables|SetCamTrans (Variables|/Game/MyContent/Blueprints/Saves/bp_CameraSaves.bp_CameraSaves_C|GetCamCord1Save _output_get)))
  (bind _output_get_4 (LocalVariables|SetStartTransform (Variables|/Game/MyContent/Blueprints/Saves/bp_CameraSaves.bp_CameraSaves_C|GetcamPlayer1 _output_get)))
  (return _output_get_2 _output_get_3 _output_get_4))