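; First-person player character that handles Enhanced Input movement and look, a crosshair widget, and camera pitch limits.
; Tick sphere-traces forward from the camera to track the current interactable and changes crosshair opacity on a hit.
; CameraInteracting saves a targeted camcorder reference to the bp_CameraSaves slot, then messages it through BPI_Interact.
; The IA_Interact input event is empty.
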(event Custom|Camera%20Interacting
  (bind _currentinteracable (Variables|Default|GetCurrentInteracable))
  ;[0.15 0.15 0.15 0.5] Event to call object interaction
  (if (Variables|Default|GetIsInteracting)
    (if (Utilities|DoesObjectImplementInterface _currentinteracable "/Game/MyContent/Blueprints/Interactible_Objects/BPI_Interact.BPI_Interact_C")
      (bind _asbp_cam_corder (Utilities|Casting|CastTobp_CamCorder _currentinteracable))
      (bind _output_get (Variables|Default|SetCameraCorder _asbp_cam_corder))
      (CallFunction|SaveCamObject _output_get)
      (Class|BPIInteract|CameraInteract(Message) _currentinteracable))))

(event Input|EnhancedActionEvents|EnhancedInputActionIA_Move
  (params (ActionValue :type Vector%202D%20Structure) (ElapsedSeconds :type Float%20%28double-precision%29) (TriggeredSeconds :type Float%20%28double-precision%29) (InputAction :type Input%20Action%20Object%20Reference :default "/Game/MyContent/Inputs/Actions/IA_Move.IA_Move"))
  (bind _returnvalue (Pawn|GetControlRotation :!class /Script/Engine.Pawn))
  ;[1 1 1] Movement Action
  (Pawn|Input|AddMovementInput (Math|Vector|GetRightVector (Math|Rotator|MakeRotator (.roll _returnvalue) 0.0 (.yaw _returnvalue))) (.x ActionValue) false)
  (Pawn|Input|AddMovementInput (Math|Vector|GetForwardVector (Math|Rotator|MakeRotator 0.0 0.0 (.yaw (Pawn|GetControlRotation :!class /Script/Engine.Pawn)))) (.y ActionValue) false))

(event Input|EnhancedActionEvents|EnhancedInputActionIA_Look
  (params (ActionValue :type Vector%202D%20Structure) (ElapsedSeconds :type Float%20%28double-precision%29) (TriggeredSeconds :type Float%20%28double-precision%29) (InputAction :type Input%20Action%20Object%20Reference :default "/Game/MyContent/Inputs/Actions/IA_Look.IA_Look"))
  ;[1 1 1] Looking Action
  (Pawn|Input|AddControllerYawInput (.x ActionValue))
  ;;[1 1 1] Negates the Y axis
  (bind _result (Math|Float|NegateFloat (.y ActionValue))
    (:%20%20
      (Pawn|Input|AddControllerPitchInput _result))))

(event Input|EnhancedActionEvents|EnhancedInputActionIA_Interact
  (params (ActionValue :type Boolean) (ElapsedSeconds :type Float%20%28double-precision%29) (TriggeredSeconds :type Float%20%28double-precision%29) (InputAction :type Input%20Action%20Object%20Reference :default "/Game/MyContent/Inputs/Actions/IA_Interact.IA_Interact"))
  ;[1 1 1] Object Inspect Interaction
)

(event EventBeginPlay
  (bind _returnvalue (Game|GetPlayerCameraManager 0))
  (Utilities|FlowControl|Sequence
    (:then_0
      ;[1 1 1] Assign Input System to Player Character
      (bind _asbp_player_controller (Utilities|Casting|CastTobp_PlayerController (Pawn|GetController)))
      (Utilities|IsValid (PlayerController|LocalPlayerSubsystems|GetEnhancedInputLocalPlayerSubsystem _asbp_player_controller)
        (:Is%20Valid
          (Input|AddMappingContext (PlayerController|LocalPlayerSubsystems|GetEnhancedInputLocalPlayerSubsystem _asbp_player_controller) "/Game/MyContent/Inputs/IMC_FPControls.IMC_FPControls" 0 "(bIgnoreAllPressedKeysUntilRelease=True,bForceImmediately=False,bNotifyUserSettings=False)"))))
    (:then_1
      ;[1 1 1] Create Crosshair
      (bind _returnvalue_2 (UserInterface|CreateWidget "/Game/MyContent/Blueprints/UI/Widgets/WBP_Crosshair.WBP_Crosshair_C"))
      (bind _output_get (Variables|Default|SetCrosshairRef _returnvalue_2))
      (UserInterface|Viewport|AddtoViewport _output_get 0))
    (:then_2
      ;[1 1 1] Setting Highest & Lowest Point for camera Y-Axis
      (Variables|/Script/Engine.PlayerCameraManager|SetViewPitchMin _returnvalue -8e+01)
      (Variables|/Script/Engine.PlayerCameraManager|SetViewPitchMax _returnvalue 25.0))))

(event EventTick
  (params (DeltaSeconds :type Float%20%28single-precision%29))
  (bind _camera (Variables|Default|GetCamera))
  (bind _crosshairref (Variables|Default|GetCrosshairRef))
  (bind _returnvalue (Transformation|GetWorldLocation _camera))
  (bind _crosshair_letter (Variables|/Game/MyContent/Blueprints/UI/Widgets/WBP_Crosshair.WBP_Crosshair_C|GetCrosshair_Letter _crosshairref))
  (bind (_outhit _returnvalue_2) (Collision|SphereTraceByChannel _returnvalue (+ _returnvalue (* (Math|Vector|GetForwardVector (Transformation|GetWorldRotation _camera)) (Variables|Default|GetInteractionDistance))) 1.0 "TraceTypeQuery3" false 0 "None" true "(R=1.000000,G=0.000000,B=0.000000,A=1.000000)" "(R=0.000000,G=1.000000,B=0.000000,A=1.000000)" 0.1))
  (if _returnvalue_2
    (Variables|Default|SetCurrentInteracable (.HitActor (Collision|BreakHitResult _outhit)))
    (Class|TextBlock|SetOpacity _crosshair_letter 0.75)
    (Variables|Default|SetIsInteracting true)
    (else
      (Class|TextBlock|SetOpacity _crosshair_letter 0.25)
      (Variables|Default|SetIsInteracting false))))

(fn ConstructionScript)

(fn SaveCamObject
  (params (CamCord :type Bp%20Cam%20Corder%20Object%20Reference))
  (bind _returnvalue (SaveGame|LoadGamefromSlot "bp_CameraSaves"))
  (bind _asbp_camera_saves (Utilities|Casting|CastTobp_CameraSaves _returnvalue))
  (Variables|/Game/MyContent/Blueprints/Saves/bp_CameraSaves.bp_CameraSaves_C|SetCamCord1 _asbp_camera_saves CamCord)
  (SaveGame|SaveGametoSlot _asbp_camera_saves "bp_CameraSaves"))