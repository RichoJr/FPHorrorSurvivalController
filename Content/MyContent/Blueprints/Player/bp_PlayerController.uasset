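; Player controller that lets the player cycle control between player characters, with remote characters viewed through an in-world camera screen.
; BeginPlay caches the character roster, the original "world" character and the game mode.
; Switching possesses the next character; for remote ones, the view stays on the world character while the screen shows a render material, otherwise it goes black.
; A separate function toggles the camcorder HUD canvas and starts the game mode's camera timer when showing it.
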(event EventBeginPlay
  (bind _outactors (Actor|GetAllActorsOfClass "/Game/MyContent/Blueprints/Player/bp_PlayerCharacter.bp_PlayerCharacter_C"))
  (Variables|Default|SetPlayerRoster _outactors)
  (bind _asbp_player_character (Utilities|Casting|CastTobp_PlayerCharacter (Game|GetPlayerCharacter 0)))
  (bind _output_get (Variables|Default|SetcurrentPlayer _asbp_player_character))
  (Variables|Default|SetworldPlayer _output_get)
  (bind _asbp_fpgame_mode (Utilities|Casting|CastToBP_FPGameMode (Game|GetGameMode)))
  (Variables|Default|SetGameMode _asbp_fpgame_mode))

(fn ConstructionScript)

(fn SwitchPlayerCharacter
  (params (Screen :type Static%20Mesh%20Component%20Object%20Reference))
  (bind _playerroster (Variables|Default|GetPlayerRoster))
  (LocalVariables|SetplayerIndex (Utilities|Array|FindItem _playerroster (Variables|Default|GetcurrentPlayer)))
  (bind _output_get (LocalVariables|SetplayerIndex (Math|Integer|SelectInt (+ (Utilities|Array|FindItem _playerroster (Variables|Default|GetcurrentPlayer)) 1) 0 (Utilities|Array|IsValidIndex _playerroster (+ (Utilities|Array|FindItem _playerroster (Variables|Default|GetcurrentPlayer)) 1)))))
  (bind _output_get_2 (Variables|Default|SetcurrentPlayer (Utilities|Array|Get(acopy) (Variables|Default|GetPlayerRoster) _output_get)))
  (Pawn|Possess _output_get_2)
  (bind _output_get_3 (Variables|Default|SetCamPlayer (== (Variables|Default|GetworldPlayer) (Variables|Default|GetcurrentPlayer))))
  (if _output_get_3
    (Rendering|Material|SetMaterial (stale _output_get_4) 0 "/Game/MyContent/Blueprints/Mats_Textures/M_BlackDebug.M_BlackDebug")
    (else
      (bind _output_get_4 (Variables|Default|SetcurrentScreen Screen))
      (Rendering|Material|SetMaterial _output_get_4 0 "/Game/MyContent/Blueprints/Mats_Textures/M_PlayerCamRender.M_PlayerCamRender")
      (Game|Player|SetViewTargetwithBlend (Variables|Default|GetworldPlayer) 0.0 "VTBlend_Linear" 0.0 false)))
  (return (Variables|Default|GetCamPlayer)))

(fn CameraScreenUIActive
  (params (CamScreenOn :type Boolean))
  (if CamScreenOn
    (bind _output_get (Variables|Default|SetDisplay (Variables|/Game/MyContent/Blueprints/Player/bp_PlayerCharacter.bp_PlayerCharacter_C|GetCrosshairRef (Variables|Default|GetcurrentPlayer))))
    (Widget|SetVisibility (Variables|/Game/MyContent/Blueprints/UI/Widgets/WBP_Crosshair.WBP_Crosshair_C|GetCamcord_Canvas _output_get) "Collapsed")
    (else
      (bind _output_get_2 (Variables|Default|SetDisplay (Variables|/Game/MyContent/Blueprints/Player/bp_PlayerCharacter.bp_PlayerCharacter_C|GetCrosshairRef (Variables|Default|GetworldPlayer))))
      (Widget|SetVisibility (Variables|/Game/MyContent/Blueprints/UI/Widgets/WBP_Crosshair.WBP_Crosshair_C|GetCamcord_Canvas _output_get_2) "HitTestInvisible")
      (Default|StartCamTimer (Variables|Default|GetGameMode)))))