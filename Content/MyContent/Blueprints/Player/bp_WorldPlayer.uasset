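; Player Blueprint that sets up a crosshair HUD and handles an interact-driven camcorder move.
; On BeginPlay it clears all widgets and adds the crosshair to the viewport.
; The interact input calls CameraInteracting and enables a Tick interpolation that eases the CameraCorder actor's location and rotation toward BpCamCordAnchor.
; A one-second timer then stops the movement, whether or not the camcorder has reached the anchor.
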(event Custom|Move%20Camera
  (Development|PrintString "Done")
  (Variables|Default|SetIsCameraMoving false))

(event Input|EnhancedActionEvents|EnhancedInputActionIA_Interact
  (params (ActionValue :type Boolean) (ElapsedSeconds :type Float%20%28double-precision%29) (TriggeredSeconds :type Float%20%28double-precision%29) (InputAction :type Input%20Action%20Object%20Reference :default "/Game/MyContent/Inputs/Actions/IA_Interact.IA_Interact"))
  (:Started
    (CallFunction|CameraInteracting)
    (Variables|Default|SetIsCameraMoving true)
    (Utilities|Time|SetTimerbyEvent (delegate Custom|Move%20Camera) 1.0)))

(event EventBeginPlay
  (|CallParentFunction)
  (Viewport|RemoveAllWidgets)
  (bind _returnvalue (UserInterface|CreateWidget "/Game/MyContent/Blueprints/UI/Widgets/WBP_Crosshair.WBP_Crosshair_C"))
  (bind _output_get (Variables|Default|SetCrosshairRef _returnvalue))
  (UserInterface|Viewport|AddtoViewport _output_get 0))

(event Collision|EventActorBeginOverlap
  (params (OtherActor :type Actor%20Object%20Reference)))

(event EventTick
  (params (DeltaSeconds :type Float%20%28single-precision%29))
  (bind _returnvalue (Utilities|Time|GetWorldDeltaSeconds))
  (bind _cameracorder (Variables|Default|GetCameraCorder))
  (bind _bp_camcordanchor (Variables|Default|Getbp_CamCordAnchor))
  (|CallParentFunction DeltaSeconds)
  (if (Variables|Default|GetIsCameraMoving)
    (Transformation|SetActorLocationAndRotation _cameracorder (Math|Interpolation|VInterpTo (Transformation|GetActorLocation _cameracorder) (Transformation|GetWorldLocation _bp_camcordanchor) _returnvalue 5.0) (Math|Interpolation|RInterpTo (Transformation|GetActorRotation (Variables|Default|GetCameraCorder)) (Transformation|GetWorldRotation _bp_camcordanchor) _returnvalue 5.0))))

(fn ConstructionScript
  (|CallParentFunction))